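; BP_SecurityMonitor is an in-world screen that shows the feed of one BP_SecurityCamera at a time.
; On BeginPlay it binds TargetTexture to a dynamic material on the Screen, gathers every security camera in the level and activates the first.
; Cameras render into that shared target through DisplayToTarget; NextCamera clears the active one and cycles to the next with wraparound.
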(event EventBeginPlay
  (CallFunction|Setup))

(fn ConstructionScript)

(fn Setup
  (bind _returnvalue (Rendering|Material|CreateDynamicMaterialInstance (Variables|Default|GetScreen) 0 (Variables|Default|GetScreenMaterial) "None" :!class /Script/Engine.PrimitiveComponent))
  (Rendering|Material|SetTextureParameterValue _returnvalue "TargetTexture" (Variables|Default|GetTargetTexture))
  (bind _outactors (Actor|GetAllActorsOfClass "/Game/SecurityCameras/Blueprints/BP_SecurityCamera.BP_SecurityCamera_C"))
  (Variables|Default|SetCameras _outactors)
  (CallFunction|SetActiveCamera))

(fn SetActiveCamera
  (params (NewIndex :type Integer))
  (bind _cameras (Variables|Default|GetCameras))
  (if (> (Utilities|Array|Length _cameras) NewIndex)
    (bind _output_get (Variables|Default|SetActiveCameraIndex NewIndex))
    (Utilities|IsValid (Utilities|Array|Get(acopy) _cameras _output_get)
      (:Is%20Valid
        (Default|DisplaytoTarget (Utilities|Array|Get(acopy) _cameras _output_get) (Variables|Default|GetTargetTexture))))))

(fn StopActiveCamera
  (bind _cameras (Variables|Default|GetCameras))
  (bind _activecameraindex (Variables|Default|GetActiveCameraIndex))
  (bind _output (Utilities|Array|Get(acopy) _cameras _activecameraindex))
  (if (> (Utilities|Array|Length _cameras) _activecameraindex)
    (Utilities|IsValid _output
      (:Is%20Valid
        (Default|ClearTarget _output)))))

(fn NextCamera
  (CallFunction|StopActiveCamera)
  (CallFunction|SetActiveCamera (Math|Integer|%(Integer) (+ (Variables|Default|GetActiveCameraIndex) 1) (Utilities|Array|Length (Variables|Default|GetCameras)))))